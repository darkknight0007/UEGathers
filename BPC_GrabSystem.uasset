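; Actor component that lets its owner pick up, carry and drop physics objects tagged "Grabable".
; It adds a PhysicsHandle to the owner at BeginPlay, and Grab toggles between releasing and a forward line trace on the Visibility channel.
; Tick holds the grabbed component at half the arm length in front of the owner.
; Debug lines visualize both the trace and the hold point.
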(event Custom|Grab
  (bind _returnvalue (Components|GetOwner))
  (bind _grabarmlength (Variables|Default|GetGrabArmLength))
  (bind _returnvalue_2 (Transformation|GetActorLocation _returnvalue))
  (bind _returnvalue_3 (Transformation|GetActorForwardVector _returnvalue))
  (bind _returnvalue_4 (* _returnvalue_3 _grabarmlength))
  (bind _returnvalue_5 (+ _returnvalue_2 _returnvalue_4))
  ;[1 1 1] Grab Event
  (if (Variables|Default|GetPickedUp)
    (CallFunction|ReleaseGrab)
    (else
      (Rendering|Debug|DrawDebugLine _returnvalue_2 _returnvalue_5 "(R=0.880000,G=0.063343,B=0.098369,A=1.000000)" 5.0 5.0)
      (bind (_outhit _returnvalue_6) (Collision|LineTraceByChannel _returnvalue_2 _returnvalue_5 "TraceTypeQuery1" false 0 "None"))
      (if _returnvalue_6
        (bind _output_get (Variables|Default|SetHitComponent (.HitComponent (Collision|BreakHitResult _outhit))))
        (if (Components|ComponentHasTag _output_get "Grabable")
          (Variables|Default|SetPickedUp true)
          (Physics|Components|PhysicsHandle|GrabComponentatLocationwithRotation (Variables|Default|GetPhysicsHandle) (Variables|Default|GetHitComponent) "None" (Transformation|GetWorldLocation (Variables|Default|GetHitComponent)) "0, 0, 0"))))))

(event Custom|ReleaseGrab
  ;[1 1 1] Release grabbed object
  (if (Variables|Default|GetPickedUp)
    (Physics|Components|PhysicsHandle|ReleaseComponent (Variables|Default|GetPhysicsHandle))
    (Variables|Default|SetPickedUp false)))

(event EventBeginPlay
  ;[1 1 1] Add PhysicsHandleComponent at runtime
  (bind _returnvalue (Game|AddComponentbyClass (Components|GetOwner) "/Script/Engine.PhysicsHandleComponent"))
  (Variables|Default|SetPhysicsHandle _returnvalue))

(event EventTick
  (params (DeltaSeconds :type Float%20%28single-precision%29))
  (bind _returnvalue (Components|GetOwner))
  (bind _grabarmlength (Variables|Default|GetGrabArmLength))
  (bind _returnvalue_2 (Transformation|GetActorLocation _returnvalue))
  (bind _returnvalue_3 (Transformation|GetActorForwardVector _returnvalue))
  (bind _returnvalue_4 (* _grabarmlength 0.5))
  (bind _returnvalue_5 (* _returnvalue_3 _returnvalue_4))
  (bind _returnvalue_6 (+ _returnvalue_2 _returnvalue_5))
  ;[1 1 1] Update the grabbed object's location
  (if (Variables|Default|GetPickedUp)
    (Physics|Components|PhysicsHandle|SetTargetLocation (Variables|Default|GetPhysicsHandle) _returnvalue_6)
    (Rendering|Debug|DrawDebugLine _returnvalue_2 _returnvalue_6 "(R=1.000000,G=0.957815,B=0.090000,A=1.000000)" 0.0 5.0)))